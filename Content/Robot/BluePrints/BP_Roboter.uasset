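; BP_Roboter is a robot actor that drives the joint pose of a skeletal UR5 arm mesh.
; Every Tick, it reads six joint angles (torso, shoulder, elbow and three hand joints) through getter functions defined outside these graphs.
; It copies each angle into the matching variable on the mesh's UR5_Skeleton_AnimBlueprint instance, repeating the cast in each Sequence branch.
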(event EventTick
  (params (DeltaSeconds :type Float%20%28single-precision%29))
  (Utilities|FlowControl|Sequence
    (:then_0
      (bind _asur5_skeleton_anim_blueprint (Utilities|Casting|CastToUR5_Skeleton_AnimBlueprint (Components|SkeletalMesh|GetAnimInstance (Variables|Default|GetRobotMesh))))
      (bind _returnvalue (Class|Robot|GetRumpfWinkel self))
      (Variables|/Game/Robot/BluePrints/UR5_Skeleton_AnimBlueprint.UR5_Skeleton_AnimBlueprint_C|SetRumpfWinkel _asur5_skeleton_anim_blueprint _returnvalue))
    (:then_1
      (bind _asur5_skeleton_anim_blueprint_2 (Utilities|Casting|CastToUR5_Skeleton_AnimBlueprint (Components|SkeletalMesh|GetAnimInstance (Variables|Default|GetRobotMesh))))
      (bind _returnvalue_2 (Class|Robot|GetSchulterWinkel self))
      (Variables|/Game/Robot/BluePrints/UR5_Skeleton_AnimBlueprint.UR5_Skeleton_AnimBlueprint_C|SetSchulterWinkel _asur5_skeleton_anim_blueprint_2 _returnvalue_2))
    (:then_2
      (bind _asur5_skeleton_anim_blueprint_3 (Utilities|Casting|CastToUR5_Skeleton_AnimBlueprint (Components|SkeletalMesh|GetAnimInstance (Variables|Default|GetRobotMesh))))
      (bind _returnvalue_3 (Class|Robot|GetEllenbogenWinkel self))
      (Variables|/Game/Robot/BluePrints/UR5_Skeleton_AnimBlueprint.UR5_Skeleton_AnimBlueprint_C|SetEllenbogenWinkel _asur5_skeleton_anim_blueprint_3 _returnvalue_3))
    (:then_3
      (bind _asur5_skeleton_anim_blueprint_4 (Utilities|Casting|CastToUR5_Skeleton_AnimBlueprint (Components|SkeletalMesh|GetAnimInstance (Variables|Default|GetRobotMesh))))
      (bind _returnvalue_4 (Class|Robot|GetHand1Winkel self))
      (Variables|/Game/Robot/BluePrints/UR5_Skeleton_AnimBlueprint.UR5_Skeleton_AnimBlueprint_C|SetHand1Winkel _asur5_skeleton_anim_blueprint_4 _returnvalue_4))
    (:then_4
      (bind _asur5_skeleton_anim_blueprint_5 (Utilities|Casting|CastToUR5_Skeleton_AnimBlueprint (Components|SkeletalMesh|GetAnimInstance (Variables|Default|GetRobotMesh))))
      (bind _returnvalue_5 (Class|Robot|GetHand2Winkel self))
      (Variables|/Game/Robot/BluePrints/UR5_Skeleton_AnimBlueprint.UR5_Skeleton_AnimBlueprint_C|SetHand2Winkel _asur5_skeleton_anim_blueprint_5 _returnvalue_5))
    (:then_5
      (bind _asur5_skeleton_anim_blueprint_6 (Utilities|Casting|CastToUR5_Skeleton_AnimBlueprint (Components|SkeletalMesh|GetAnimInstance (Variables|Default|GetRobotMesh))))
      (bind _returnvalue_6 (Class|Robot|GetHand3Winkel self))
      (Variables|/Game/Robot/BluePrints/UR5_Skeleton_AnimBlueprint.UR5_Skeleton_AnimBlueprint_C|SetHand3Winkel _asur5_skeleton_anim_blueprint_6 _returnvalue_6))))

(fn ConstructionScript)